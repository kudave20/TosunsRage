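; Parent Blueprint for Tosun, an enemy that chases the player and can be shot dead.
; Tick turns the capsule toward the player and steps the actor forward a fixed amount per frame, without sweep or pathfinding.
; Capsule overlaps with Glock, MP5 or AK74 tracer rounds subtract per-weapon damage from Health.
; At zero, DeathTosun ragdolls the mesh, removes collision, stops Tick and plays kill sounds before destruction; health-widget setup is unconnected.
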(event `self.ReceiveTick`
  (params (DeltaSeconds :type "Float (single-precision)"))
  (bind _capsulecomponent (`self.CapsuleComponent`))
  ;[1 1 1] AI Movement
  (`|ExecutionSequence`
    (:`then_1`
      (`/Engine/EditorBlueprintResources/StandardMacros.IsValid` _capsulecomponent
        (:`Is Valid`
          (`|ExecutionSequence`
            (:`then_0`
              (`SceneComponent.K2_SetWorldRotation` _capsulecomponent (`KismetMathLibrary.FindLookAtRotation` (`self.K2_GetActorLocation`) (`self.K2_GetActorLocation` (`GameplayStatics.GetPlayerCharacter` 0))) false false))
            (:`then_1`
              (`self.K2_SetActorLocation` (+ (`self.K2_GetActorLocation`) (* (`SceneComponent.GetForwardVector` (`self.CapsuleComponent`)) 2.0))))))))))

(event `self.CapsuleComponent.OnComponentBeginOverlap`
  (params (OverlappedComponent :type "PrimitiveComponent Object Reference") (OtherActor :type "Actor Object Reference") (OtherComp :type "PrimitiveComponent Object Reference") (OtherBodyIndex :type Integer) (bFromSweep :type Boolean) (SweepResult :type "HitResult Structure (by ref)"))
  ;[1 1 1] Health
  (`|ExecutionSequence`
    (:`then_0`
      (cast `/Game/FirstPerson/Blueprints/Weapons/Glock26_TracerRound_BP` OtherActor)
      (set `self.Health` (- (`self.Health`) (`self.GlockDamage`)))
      (if (>= 0 (`self.Health`))
        (`self.DeathTosun` :!label _label)
        (`KismetSystemLibrary.Delay` 5.0)
        (`self.K2_DestroyActor`)
        (else
          (`GameplayStatics.PlaySound2D` "/Game/Tosun/Sounds/A_Hit_Cue.A_Hit_Cue" 1.0 1.0 0.0 null null :!label _label_2))))
    (:`then_1`
      (cast `/Game/FirstPerson/Blueprints/Weapons/MP5_TracerRound_BP` OtherActor)
      (set `self.Health` (- (`self.Health`) (`self.MP5Damage`)))
      (if (>= 0 (`self.Health`))
        (goto _label)
        (else
          (goto _label_2))))
    (:`then_2`
      (cast `/Game/FirstPerson/Blueprints/Weapons/AK74_TracerRound_BP` OtherActor)
      (set `self.Health` (- (`self.Health`) (`self.AK74Damage`)))
      (if (>= 0 (`self.Health`))
        (goto _label)
        (else
          (goto _label_2))))))

(event `Body`
  ;[1 1 1] Health
)

(fn `CastToCharacter`
  (set `self.As First Person Character` (cast `/Game/FirstPerson/Blueprints/Player/FPSPawn_BP` (`GameplayStatics.GetPlayerCharacter` 0) :!pure true)))

(fn `TosunHealth`
  (params (Object :type "Object Object Reference") (Object2 :type "Object Object Reference") (Object3 :type "Object Object Reference")))

(fn `UserConstructionScript`)