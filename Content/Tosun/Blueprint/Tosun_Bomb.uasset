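; Tosun_Bomb is a suicide-bomber style character that self-explodes when the FPSPawn_BP pawn enters its AttackCollision.
; On overlap it spawns an explosion effect actor, switches its mesh to physics simulation, removes its capsule and trigger, then destroys itself after a delay.
; InRange tracks the overlap, and a separate Body event removes the Fire component.
; This graph applies no damage directly.
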(event `self.AttackCollision.OnComponentBeginOverlap`
  (params (OverlappedComponent :type "PrimitiveComponent Object Reference") (OtherActor :type "Actor Object Reference") (OtherComp :type "PrimitiveComponent Object Reference") (OtherBodyIndex :type Integer) (bFromSweep :type Boolean) (SweepResult :type "HitResult Structure (by ref)"))
  ;[1 1 1] Self Explosion
  (cast `/Game/FirstPerson/Blueprints/Player/FPSPawn_BP` OtherActor)
  (set `self.InRange` true)
  (if (`self.InRange`)
    (`|SpawnActorFromClass` "/Game/StarterContent/Blueprints/Blueprint_Effect_Explosion.Blueprint_Effect_Explosion_C" (`self.GetTransform`) "Undefined" "OverrideRootScale" null null)
    (`PrimitiveComponent.SetSimulatePhysics` (`self.Mesh`) true)
    (`ActorComponent.K2_DestroyComponent` (`self.CapsuleComponent`))
    (`ActorComponent.K2_DestroyComponent` (`self.AttackCollision`))
    (`KismetSystemLibrary.Delay` 10.0)
    (`self.K2_DestroyActor`)))

(event `self.AttackCollision.OnComponentEndOverlap`
  (params (OverlappedComponent :type "PrimitiveComponent Object Reference") (OtherActor :type "Actor Object Reference") (OtherComp :type "PrimitiveComponent Object Reference") (OtherBodyIndex :type Integer))
  ;[1 1 1] Self Explosion
  (cast `/Game/FirstPerson/Blueprints/Player/FPSPawn_BP` OtherActor)
  (set `self.InRange` false))

(event `self.Body`
  (`ActorComponent.K2_DestroyComponent` (`self.Fire`)))

(fn `UserConstructionScript`
  (`parent.UserConstructionScript`))