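; Tosun_Big is a Blueprint for a large Tosun character that plays an attack animation while the player's FPSPawn_BP is within range.
; Overlap begin and end on AttackCollision set an InRange flag, and the attack montage repeats after a one-second pause following each completion while that flag holds.
; A separate Body event destroys the Smoke component.
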(event `self.AttackCollision.OnComponentBeginOverlap`
  (params (OverlappedComponent :type "PrimitiveComponent Object Reference") (OtherActor :type "Actor Object Reference") (OtherComp :type "PrimitiveComponent Object Reference") (OtherBodyIndex :type Integer) (bFromSweep :type Boolean) (SweepResult :type "HitResult Structure (by ref)"))
  ;[1 1 1] Attack Animation
  (cast `/Game/FirstPerson/Blueprints/Player/FPSPawn_BP` OtherActor)
  (set `self.InRange` true)
  (if (`self.InRange`) :!label _label
    (`|PlayMontage` (`self.Mesh`) "/Game/Tosun/Animation/BigTosun_Attack_Anim_mixamo_com_Montage.BigTosun_Attack_Anim_mixamo_com_Montage"
      (:`OnCompleted`
        (`KismetSystemLibrary.Delay` 1.0)
        (goto _label)))))

(event `self.AttackCollision.OnComponentEndOverlap`
  (params (OverlappedComponent :type "PrimitiveComponent Object Reference") (OtherActor :type "Actor Object Reference") (OtherComp :type "PrimitiveComponent Object Reference") (OtherBodyIndex :type Integer))
  ;[1 1 1] Attack Animation
  (cast `/Game/FirstPerson/Blueprints/Player/FPSPawn_BP` OtherActor)
  (set `self.InRange` false))

(event `self.Body`
  (`ActorComponent.K2_DestroyComponent` (`self.Smoke`)))

(fn `UserConstructionScript`
  (`parent.UserConstructionScript`))